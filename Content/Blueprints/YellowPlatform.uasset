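; YellowPlatform is a platform Blueprint that toggles between solid and passable.
; The ChangeStatus event calls SetCollision, which flips the IsCollisionEnabled flag on each call.
; SetCollision switches the Cube's collision profile between BlockAllDynamic and NoCollision, swapping its material to match: M_YellowPlatform when solid, CubeMaterial when passable.
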(event EventChangeStatus
  (CallFunction|SetCollision))

(fn ConstructionScript)

(fn SetCollision
  (bind _cube (Variables|Default|GetCube))
  (if (Variables|Default|GetIsCollisionEnabled)
    (Collision|SetCollisionProfileName _cube "NoCollision" true :!class /Script/Engine.PrimitiveComponent)
    (Rendering|Material|SetMaterial _cube 0 "/Game/Geometry/Meshes/CubeMaterial.CubeMaterial")
    (Variables|Default|SetIsCollisionEnabled (not (Variables|Default|GetIsCollisionEnabled)))
    (else
      (Collision|SetCollisionProfileName _cube "BlockAllDynamic" true :!class /Script/Engine.PrimitiveComponent)
      (Rendering|Material|SetMaterial _cube 0 "/Game/StarterContent/Materials/M_YellowPlatform.M_YellowPlatform")
      (Variables|Default|SetIsCollisionEnabled (not (Variables|Default|GetIsCollisionEnabled))))))